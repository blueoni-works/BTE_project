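; Interactable item Blueprint, named as the master item, that shows an interaction hint when BP_Character comes within range.
; Sphere overlap, gated by CanInteract, creates a UI_Interact widget, plays its PopUp animation, applies an outline overlay material and sets CanPressE.
; Leaving reverses these, removing the widget after a short delay.
; CanReceiveTrace repeats the hint logic behind HintVisible checks and prints a debug string; no input handling lives here.
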(event `self.Sphere.OnComponentBeginOverlap`
  (params (OverlappedComponent :type "PrimitiveComponent Object Reference") (OtherActor :type "Actor Object Reference") (OtherComp :type "PrimitiveComponent Object Reference") (OtherBodyIndex :type Integer) (bFromSweep :type Boolean) (SweepResult :type "HitResult Structure (by ref)"))
  (bind _widget (`self.Widget`))
  (cast `/Game/Programming/Blueprints/BP_Character` OtherActor)
  (if (`self.CanInteract`)
    (bind _returnvalue (`|CreateWidget` "/Game/Programming/Widgets/UI_Interact.UI_Interact_C"))
    (bind _output_get (set `self.InteractionWdget` _returnvalue))
    (`WidgetComponent.SetWidget` _widget _output_get)
    (`SceneComponent.SetVisibility` _widget true false)
    (bind _interactionwdget (`self.InteractionWdget`)
      (:`then`
        (if (not (`self.HintVisible`))
          (`UserWidget.PlayAnimation` _interactionwdget (`/Game/Programming/Widgets/UI_Interact.PopUp` _interactionwdget) 0.0 1 "Forward" 1.5 false)
          (set `self.HintVisible` true)
          (`MeshComponent.SetOverlayMaterial` (`self.StaticMesh`) "/Game/Programming/Materials/M_Outline.M_Outline" false 0)
          (set `self.CanPressE` true)))
      (:`else`))))

(event `self.Sphere.OnComponentEndOverlap`
  (params (OverlappedComponent :type "PrimitiveComponent Object Reference") (OtherActor :type "Actor Object Reference") (OtherComp :type "PrimitiveComponent Object Reference") (OtherBodyIndex :type Integer))
  (cast `/Game/Programming/Blueprints/BP_Character` OtherActor)
  (if (`self.CanInteract`)
    (bind _interactionwdget (`self.InteractionWdget`)
      (:`then`
        (if (`self.HintVisible`)
          (`UserWidget.PlayAnimation` _interactionwdget (`/Game/Programming/Widgets/UI_Interact.PopUp` _interactionwdget) 0.0 1 "Reverse" 1.5 false)
          (set `self.HintVisible` false)
          (set `self.CanPressE` false)
          (`MeshComponent.SetOverlayMaterial` (`self.StaticMesh`) null false 0))
        (`KismetSystemLibrary.Delay` 0.15)
        (`Widget.RemoveFromParent` (`self.InteractionWdget`))
        (set `self.InteractionWdget` null)
        (`SceneComponent.SetVisibility` (`self.Widget`) false false))
      (:`else`))))

(event `/Game/Programming/Blueprints/BPI_Interaction.Can Receive Trace`
  (params (`Can interact` :type Boolean))
  (`KismetSystemLibrary.PrintString` "Hello")
  (if (`self.CanInteract`)
    (if `Can interact`
      (bind _interactionwdget (`self.InteractionWdget`)
        (:`then`
          (if (`self.HintVisible`)
            (`UserWidget.PlayAnimation` _interactionwdget (`/Game/Programming/Widgets/UI_Interact.PopUp` _interactionwdget) 0.0 1 "Forward" 1.5 false)
            (set `self.HintVisible` true)
            (`MeshComponent.SetOverlayMaterial` (`self.StaticMesh`) "/Game/Programming/Materials/M_Outline.M_Outline" false 0)
            (set `self.CanPressE` true)))
        (:`else`))
      (else
        (bind _interactionwdget_2 (`self.InteractionWdget`)
          (:`then`
            (if (`self.HintVisible`)
              (`UserWidget.PlayAnimation` _interactionwdget_2 (`/Game/Programming/Widgets/UI_Interact.PopUp` _interactionwdget_2) 0.0 1 "Reverse" 1.5 false)
              (set `self.HintVisible` false)
              (`MeshComponent.SetOverlayMaterial` (`self.StaticMesh`) null false 0)
              (set `self.CanPressE` false)))
          (:`else`))))))

(fn `UserConstructionScript`)